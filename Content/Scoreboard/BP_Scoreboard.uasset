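; BP_Scoreboard is an in-world scoreboard actor that hosts a widget component displaying score information.
; On BeginPlay it checks the level name: in MainLevel it hands its target manager reference to WIDGET_Scoreboard.
; In other levels it passes the alien target manager reference to WIDGET_AlienScoreboard1 instead.
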(event EventBeginPlay
  (bind _returnvalue (Game|GetCurrentLevelName true))
  (if (Utilities|Enum|Equal(Enum) _returnvalue "MainLevel")
    (bind _aswidget_scoreboard (Utilities|Casting|CastToWIDGET_Scoreboard (UserInterface|GetUserWidgetObject (Variables|Default|GetWidget))))
    (Variables|/Game/Scoreboard/WIDGET_Scoreboard.WIDGET_Scoreboard_C|SetTargetManagerRef _aswidget_scoreboard (Variables|Default|GetTargetManagerRef))
    (else
      (bind _aswidget_alien_scoreboard_1 (Utilities|Casting|CastToWIDGET_AlienScoreboard1 (UserInterface|GetUserWidgetObject (Variables|Default|GetWidget))))
      (Variables|/Game/Scoreboard/WIDGET_AlienScoreboard1.WIDGET_AlienScoreboard1_C|SetTargetManagerRef _aswidget_alien_scoreboard_1 (Variables|Default|GetalientarmanRef)))))

(event Collision|EventActorBeginOverlap
  (params (OtherActor :type Actor%20Object%20Reference)))

(event EventTick
  (params (DeltaSeconds :type Float%20%28single-precision%29)))

(fn ConstructionScript)