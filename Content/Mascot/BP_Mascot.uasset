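; BP_Mascot is the mascot's voice, playing narrative dialogue for intro, acts and finale, including alien variants, plus shot reactions.
; PlayDialogueArray steps through each array's audio cues on one Audio component, delaying by each line's duration plus padding until an invalid cue or skip flag.
; The menu's SkipDialogue takes effect after the current delay.
; Reactions play only when dialogue has finished; knockdowns trigger one randomly, and some reaction events are empty.
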(event Custom|Play_Dialogue_Intro
  ;[1 1 1] Narrative Dialogue
  (CallFunction|PlayDialogueArray (Variables|Default|GetDial_Intro)))

(event Custom|React_ShotByPlayer
  ;[1 1 1] Reaction Dialogue
)

(event Custom|SkipDialogue
  ;[1 1 1] Used by Menu
  (Variables|Default|SetDialogueArrayFinished true))

(event Custom|Play_Dialogue_Finale
  ;[1 1 1] Narrative Dialogue
  (CallFunction|PlayDialogueArray (Variables|Default|GetDial_Finale)))

(event Custom|Play_dial_alienIntro
  ;[1 1 1] Narrative Dialogue
  (CallFunction|PlayDialogueArray (Variables|Default|Getalien_intro)))

(event Custom|play_dia_alienact1
  ;[1 1 1] Narrative Dialogue
  (CallFunction|PlayDialogueArray (Variables|Default|Getalien_act1)))

(event Custom|play_dia_alienact2
  ;[1 1 1] Narrative Dialogue
  (CallFunction|PlayDialogueArray (Variables|Default|Getalien_act2)))

(event Custom|React_GoodShot
  ;[1 1 1] Reaction Dialogue
  (CallFunction|PlayReaction "/Game/Audio/Dialogue/VO/Reaction/CUE_React_GoodShot.CUE_React_GoodShot"))

(event Custom|React_PlayerMissedShot
  ;[1 1 1] Reaction Dialogue
)

(event Custom|Play_Dialogue_Act1
  ;[1 1 1] Narrative Dialogue
  (CallFunction|PlayDialogueArray (Variables|Default|GetDial_Act1)))

(event Custom|PlayDialogueArray
  (params (DialogueArray :type Array%20of%20Struct%20Dialogue%20Structures))
  (bind _audio (Variables|Default|GetAudio))
  (Audio|Components|Audio|Stop (Variables|Default|GetAudio))
  (Variables|Default|SetArrayIndex 0)
  (Variables|Default|SetDialogueArrayFinished false)
  (Utilities|IsValid (.AudioCue (Utilities|Struct|BreakStruct_Dialogue (Utilities|Array|Get(acopy) DialogueArray (Variables|Default|GetArrayIndex)))) :!label _label
    (:Is%20Valid
      (Audio|Components|Audio|SetSound _audio (.AudioCue (Utilities|Struct|BreakStruct_Dialogue (Utilities|Array|Get(acopy) DialogueArray (Variables|Default|GetArrayIndex)))))
      (Audio|Components|Audio|Play _audio 0.0)
      (Utilities|FlowControl|Delay (+ (.Duration (Utilities|Struct|BreakStruct_Dialogue (Utilities|Array|Get(acopy) DialogueArray (Variables|Default|GetArrayIndex)))) 0.5))
      (Math|Integer|IncrementInt (Variables|Default|GetArrayIndex)
        (:%20%20
          (if (not (Variables|Default|GetDialogueArrayFinished))
            (goto _label)))))
    (:Is%20Not%20Valid
      (Variables|Default|SetDialogueArrayFinished true))))

(event Custom|Play_Dialogue_Act2
  ;[1 1 1] Narrative Dialogue
  (CallFunction|PlayDialogueArray (Variables|Default|GetDial_Act2)))

(event Custom|Play_Dialogue_Act3
  ;[1 1 1] Narrative Dialogue
  (CallFunction|PlayDialogueArray (Variables|Default|GetDial_Act3)))

(event Custom|play_dia_alienfinale
  ;[1 1 1] Narrative Dialogue
  (CallFunction|PlayDialogueArray (Variables|Default|Getalien_Finale)))

(event Custom|Play_Reaction
  (params (SoundCue :type Sound%20Cue%20Object%20Reference))
  (bind _audio (Variables|Default|GetAudio))
  (if (Variables|Default|GetDialogueArrayFinished)
    (Audio|Components|Audio|Stop (Variables|Default|GetAudio))
    (Audio|Components|Audio|SetSound _audio SoundCue)
    (Audio|Components|Audio|Play _audio 0.0)))

(event EventKnockDown
  (params (CountsForPoints :type Boolean))
  ;[1 1 1] Reaction Dialogue
  (if (== (Math|Random|RandomIntegerinRange 0 2) 0)
    (CallFunction|PlayReaction (Variables|Default|GetReac_dial))))

(fn ConstructionScript)