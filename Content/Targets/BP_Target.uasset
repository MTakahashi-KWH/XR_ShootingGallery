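; BP_Target is a moving shooting-gallery style target that awards points through a target manager when knocked down.
; BeginPlay applies the chosen mesh and starts a fast looping timer; UpdatePosition slides it along its right vector, and SwitchDirection reverses Speed.
; spawncreature stores the death sound and occasionally plays a spawn sound.
; KnockDown optionally scores and plays that death sound, disables collision, rotates via timeline, pings and destroys the actor after a short delay.
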(event Custom|UpdatePosition
  (Transformation|AddActorWorldOffset (* (Transformation|GetActorRightVector) (Variables|Default|GetSpeed))))

(event Custom|spawn%20creature
  (params (spawn%20noise :type Sound%20Cue%20Object%20Reference) (death%20noise :type Sound%20Cue%20Object%20Reference))
  (Variables|Default|Setdeathnoise death%20noise)
  (if (== (Class|KismetMathLibrary|ToInt64(Integer) (Math|Random|RandomIntegerinRange 0 4)) 0)
    (Audio|PlaySoundatLocation spawn%20noise "0, 0, 0" "0, 0, 0" 1.0 1.0 0.0 0 0 0)))

(event EventBeginPlay
  (Utilities|Time|SetTimerbyEvent (EventDispatchers|CreateEvent :!event Custom|UpdatePosition) 0.01 true)
  (Components|StaticMesh|SetStaticMesh (Variables|Default|GetTargetMesh) (Variables|Default|GetChosenTargetMesh)))

(event EventKnockDown
  (params (CountsForPoints :type Boolean))
  (Utilities|FlowControl|Sequence
    (:then_0
      (if CountsForPoints
        (Default|AddPoints (Variables|Default|GetTargetManagerRef) 175)
        ;[1 1 1] ADD SOUND HERE
        (Audio|PlaySoundatLocation (Variables|Default|Getdeathnoise) "0, 0, 0" "0, 0, 0" 1.0 1.0 0.0 0 0 0)))
    (:then_1
      (Collision|SetCollisionEnabled (Variables|Default|GetTargetMesh) "NoCollision")
      (bind _yrotation (Timeline|KnockDownAnimTimeline Play)
        (:Update
          (Transformation|SetActorRotation (Math|Rotator|MakeRotator 0.0 _yrotation 0.0)))))
    (:then_2
      (Utilities|FlowControl|Delay 0.2)
      (Actor|DestroyActor))
    (:then_3
      (Audio|PlaySoundatLocation "/Game/Audio/target/CUE_target_hitping.CUE_target_hitping" (Transformation|GetActorLocation) "0, 0, 0" 1.0 1.0 0.0 0 0 0))))

(fn ConstructionScript)

(fn SwitchDirection
  (Variables|Default|SetSpeed (* (Variables|Default|GetSpeed) -1.0)))